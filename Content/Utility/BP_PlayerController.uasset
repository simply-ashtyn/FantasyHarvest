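; Player controller Blueprint that owns the player HUD and toggles the inventory menu.
; On BeginPlay, the local controller creates WBP_PlayerHUD and adds it to the viewport.
; The Inventory input action flips InventoryOpen, calling the HUD to display or close the player menu while switching between Game and UI input with a visible cursor and game-only input.
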(event EventBeginPlay
  (if (Pawn|IsLocalPlayerController)
    (bind _returnvalue (UserInterface|CreateWidget "/Game/Widgets/WBP_PlayerHUD.WBP_PlayerHUD_C"))
    (bind _output_get (Variables|Default|SetHUD _returnvalue))
    (UserInterface|Viewport|AddtoViewport _output_get 0)))

(event EventTick
  (params (DeltaSeconds :type Float%20%28single-precision%29)))

(event Input|ActionEvents|InputActionInventory
  (params (Key :type Key%20Structure :default "None"))
  (bind _hud (Variables|Default|GetHUD))
  (:Pressed
    (if (not (Variables|Default|GetbInventoryOpen))
      (Default|DisplayPlayerMenu _hud)
      (Variables|Default|SetbInventoryOpen true)
      (Input|SetInputModeGameandUI self (Variables|Default|GetHUD) "LockAlways" false false)
      (Variables|Default|SetbShowMouseCursor true)
      (else
        (Default|ClosePlayerMenu _hud)
        (Variables|Default|SetbInventoryOpen false)
        (Input|SetInputModeGameOnly self false)
        (Variables|Default|SetbShowMouseCursor false)))))

(fn ConstructionScript)