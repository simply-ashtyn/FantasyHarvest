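; AC_InventorySystem is a player component providing a slot-based inventory and interaction with nearby actors.
; A per-tick sphere trace picks LookAtActor, and Interact sends it to the server for item, plot or generic handling.
; Items stack up to DT_ItemData limits, and server-side transfers swap or merge slots, then multicast updates.
; RemoveFromInventory and CareForCrops are empty stubs, and merging discards any overflow beyond the stack limit.
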(event Custom|MC_Update
  (Default|CallOnInventoryUpdated))

(event Custom|OnLocalInteract
  (params (TargetActor :type Actor%20Object%20Reference) (Interactor :type Actor%20Object%20Reference))
  (Class|BIInteractable|Interactwith(Message) TargetActor (.AsBP%20Base%20Player (Utilities|Casting|CastToBP_BasePlayer Interactor))))

(event Custom|Server_Interact
  (params (Target :type Actor%20Object%20Reference))
  (bind _returnvalue (Components|GetOwner))
  (bind _returnvalue_2 (Actor|GetComponentbyClass Target "/Game/ComponentSystems/Inventory/AC_ItemDataComponent.AC_ItemDataComponent_C"))
  (bind _asbp_base_player (Utilities|Casting|CastToBP_BasePlayer _returnvalue))
  (Utilities|IsValid _returnvalue_2
    (:Is%20Valid
      (Class|BIInteractable|Interactwith(Message) _returnvalue_2 (.AsBP%20Base%20Player (Utilities|Casting|CastToBP_BasePlayer (Components|GetOwner)))))
    (:Is%20Not%20Valid
      (Utilities|IsValid (Actor|GetComponentbyClass Target "/Game/ComponentSystems/Farming/AC_PlotSystem.AC_PlotSystem_C")
        (:Is%20Valid
          (CallFunction|CareforCrops))
        (:Is%20Not%20Valid
          (Actor|SetOwner Target (Pawn|GetController _asbp_base_player))
          (CallFunction|OnLocalInteract Target _asbp_base_player))))))

(event Custom|SERVER_TransferSlots
  (params (Source%20Index :type Integer) (Destination%20Index :type Integer) (Source%20Inventory :type AC%20Inventory%20System%20Object%20Reference))
  (CallFunction|TransferSlots Source%20Index Destination%20Index Source%20Inventory))

(event EventBeginPlay
  (Utilities|Array|Resize (Variables|Inventory|GetContent) (Variables|Inventory|GetInventorySize)))

(event EventTick
  (params (DeltaSeconds :type Float%20%28single-precision%29))
  (CallFunction|InteractionTrace))

(event Input|ActionEvents|InputActionInteract
  (params (Key :type Key%20Structure :default "None"))
  (:Pressed
    (bind _lookatactor (Variables|Inventory|GetLookAtActor)
      (:then
        (CallFunction|ServerInteract _lookatactor))
      (:else))))

(event Input|ActionEvents|InputActionDebugPrintContents
  (params (Key :type Key%20Structure :default "None"))
  (:Pressed
    (CallFunction|DebugPrintContents)))

(fn AddtoInventory
  (params (ItemName :type Name) (Quantity :type Integer))
  (LocalVariables|SetLocal_QuantityRemaining Quantity)
  (while (and (> (LocalVariables|GetLocal_QuantityRemaining) 0) (not (LocalVariables|GetLocal_bHasFailed)))
    (bind (_index _bslotfound) (CallFunction|FindSlot ItemName))
    (if _bslotfound
      (CallFunction|AddtoStack _index 1)
      (Math|Integer|DecrementInt (LocalVariables|GetLocal_QuantityRemaining))
      (elif (.bHasEmptySlot (CallFunction|AnyEmptySlots))
        (bind _success (CallFunction|CreateStack ItemName 1))
        (if _success
          (Math|Integer|DecrementInt (LocalVariables|GetLocal_QuantityRemaining))
          (else
            (LocalVariables|SetLocal_bHasFailed true :!label _label)))
        (else
          (goto _label)))))
  (return (not (LocalVariables|GetLocal_bHasFailed)) (LocalVariables|GetLocal_QuantityRemaining)))

(fn RemovefromInventory)

(fn AddtoStack
  (params (Index :type Integer) (Quantity :type Integer))
  (bind _content (Variables|Inventory|GetContent))
  (bind _output (Utilities|Array|Get(acopy) _content Index))
  (Utilities|Array|SetArrayElem _content Index (Utilities|Struct|MakeF_SlotStruct (.itemname _output) (+ (.quantity _output) Quantity))))

(fn InteractionTrace
  (bind _returnvalue (Game|GetPlayerCharacter 0))
  (bind _returnvalue_2 (Transformation|GetActorLocation _returnvalue))
  (bind _returnvalue_3 (- _returnvalue_2 "0.000000,0.000000,65.000000"))
  (bind (_outhit _returnvalue_4) (Collision|SphereTraceByChannel _returnvalue_3 _returnvalue_3 (Variables|Inventory|GetInteractionRange) "TraceTypeQuery3" false (Utilities|Array|MakeArray (Components|GetOwner)) "None"))
  (if _returnvalue_4
    (if (!= (.HitActor (Collision|BreakHitResult _outhit)) (Variables|Inventory|GetLookAtActor))
      (bind _output_get (Variables|Inventory|SetLookAtActor (.HitActor (Collision|BreakHitResult _outhit))))
      (bind _message (Class|BIInteractable|Lookat(Message) _output_get))
      (Development|PrintString (Utilities|String|ToString(Text) _message)))
    (else
      (Variables|Inventory|SetLookAtActor 0))))

(fn DebugPrintContents
  (for (_array_element _array_index) (Variables|Inventory|GetContent)
    (Development|PrintString (Utilities|String|Append (Utilities|String|ToString(Integer) _array_index) " : " (Utilities|String|ToString(Name) (.ItemName (Utilities|Struct|BreakF_SlotStruct _array_element))) " = " (Utilities|String|ToString(Integer) (.Quantity (Utilities|Struct|BreakF_SlotStruct _array_element)))))))

(fn FindSlot
  (params (ItemName :type Name))
  (for (_array_element _array_index) (Variables|Inventory|GetContent)
    (if (== (.ItemName (Utilities|Struct|BreakF_SlotStruct _array_element)) ItemName)
      (if (< (.Quantity (Utilities|Struct|BreakF_SlotStruct _array_element)) (CallFunction|GetMaxStackSize ItemName))
        (return _array_index true))))
  (return -1 false))

(fn GetMaxStackSize
  (params (ItemName :type Name))
  (bind _returnvalue (Utilities|GetDataTableRow "/Game/ComponentSystems/Inventory/DT_ItemData.DT_ItemData" ItemName)
    (:then
      (return (.StackSize (Utilities|Struct|BreakF_ItemStruct _returnvalue))))
    (:RowNotFound
      (return -1))))

(fn AnyEmptySlots
  (for (_array_element _array_index) (Variables|Inventory|GetContent)
    (if (== (.Quantity (Utilities|Struct|BreakF_SlotStruct _array_element)) 0)
      (return true _array_index)))
  (return false -1))

(fn CreateStack
  (params (ItemName :type Name) (Quantity :type Integer))
  (bind (_bhasemptyslot _emptyindex) (CallFunction|AnyEmptySlots))
  (if _bhasemptyslot
    (Utilities|Array|SetArrayElem (Variables|Inventory|GetContent) _emptyindex (Utilities|Struct|MakeF_SlotStruct ItemName Quantity))
    (return true)
    (else
      (return false))))

(fn TransferSlots
  (params (SourceIndex :type Integer) (DestinationIndex :type Integer) (SourceInventory :type AC%20Inventory%20System%20Object%20Reference))
  (bind _content (Variables|Inventory|GetContent))
  (bind _output (Utilities|Array|Get(acopy) _content DestinationIndex))
  (LocalVariables|SetLocalSlotContent (Utilities|Array|Get(acopy) (Variables|AC_InventorySystem_C|GetContent SourceInventory) SourceIndex))
  (if (not (< DestinationIndex 0))
    (if (== (.ItemName (Utilities|Struct|BreakF_SlotStruct (LocalVariables|GetLocalSlotContent))) (.ItemName (Utilities|Struct|BreakF_SlotStruct _output)))
      (Utilities|Array|SetArrayElem (Variables|AC_InventorySystem_C|GetContent SourceInventory) SourceIndex (Utilities|Struct|MakeF_SlotStruct (select (> (Math|Integer|Clamp(Integer) (- (+ 0 0) (CallFunction|GetMaxStackSize (.itemname (LocalVariables|GetLocalSlotContent)))) 0 (CallFunction|GetMaxStackSize (.itemname (LocalVariables|GetLocalSlotContent)))) 0) (.itemname (LocalVariables|GetLocalSlotContent)) "None") (Math|Integer|Clamp(Integer) (- (+ 0 0) (CallFunction|GetMaxStackSize (.itemname (LocalVariables|GetLocalSlotContent)))) 0 (CallFunction|GetMaxStackSize (.itemname (LocalVariables|GetLocalSlotContent))))))
      (Utilities|Array|SetArrayElem (Variables|Inventory|GetContent) DestinationIndex (Utilities|Struct|MakeF_SlotStruct (.itemname (LocalVariables|GetLocalSlotContent)) (Math|Integer|Clamp(Integer) (+ (.quantity (LocalVariables|GetLocalSlotContent)) (.quantity (Utilities|Array|Get(acopy) (Variables|Inventory|GetContent) DestinationIndex))) 0 (CallFunction|GetMaxStackSize (.itemname (LocalVariables|GetLocalSlotContent))))))
      (CallFunction|MCUpdate)
      (CallFunction|MCUpdate SourceInventory)
      (else
        (Utilities|Array|SetArrayElem (Variables|AC_InventorySystem_C|GetContent SourceInventory) SourceIndex _output)
        (Utilities|Array|SetArrayElem (Variables|Inventory|GetContent) DestinationIndex (LocalVariables|GetLocalSlotContent))
        (CallFunction|MCUpdate)
        (CallFunction|MCUpdate SourceInventory)))))

(fn CareforCrops)