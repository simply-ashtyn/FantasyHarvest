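; Base spell actor that moves by projectile movement and takes its stats from a spell data table.
; The construction script looks up the row named by SpellInfo.SpellName in DT_SpellDataTable, overwrites SpellInfo with it, and applies its speed as the projectile's initial and maximum speed.
; BeginPlay sets a short lifespan so the spell destroys itself; this Blueprint has no active overlap or hit logic.
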(event EventBeginPlay
  (Actor|SetLifeSpan 2.0))

(event Collision|EventActorBeginOverlap
  (params (OtherActor :type Actor%20Object%20Reference)))

(event EventTick
  (params (DeltaSeconds :type Float%20%28single-precision%29)))

(fn ConstructionScript
  (bind _projectilemovement (Variables|Default|GetProjectileMovement))
  (bind _returnvalue (Utilities|GetDataTableRow "/Game/ComponentSystems/Magic/DT_SpellDataTable.DT_SpellDataTable" (Utilities|String|StringToName (Utilities|String|ToString(Byte) (.spellname (Variables|Default|GetSpellInfo)))))
    (:then
      (bind _output_get (Variables|Default|SetSpellInfo _returnvalue))
      (Variables|/Script/Engine.ProjectileMovementComponent|SetInitialSpeed _projectilemovement (.Speed (Utilities|Struct|BreakF_SpellData _output_get)))
      (Variables|/Script/Engine.ProjectileMovementComponent|SetMaxSpeed _projectilemovement (.Speed (Utilities|Struct|BreakF_SpellData _output_get))))))