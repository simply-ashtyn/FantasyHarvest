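; BP_BasePlayer is the base player Blueprint, which casts spells through the Gameplay Ability System and opens a spellbook UI.
; BeginPlay grants the water and harvest spell abilities, which debug keys T and R activate by class.
; Debug key F toggles a lazily created, reused spellbook widget, switching input mode and mouse cursor with it.
; The spellbook toggle is ignored while the inventory is open.
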(event EventBeginPlay
  (GameplayAbilities|GiveAbility (Variables|Default|GetAbilitySystem) "/Game/ComponentSystems/Magic/Farming/BP_WaterSpell.BP_WaterSpell_C" 0 -1)
  (GameplayAbilities|GiveAbility (Variables|Default|GetAbilitySystem) "/Game/ComponentSystems/Magic/Farming/BP_HarvestSpell.BP_HarvestSpell_C" 0 -1))

(event Collision|EventActorBeginOverlap
  (params (OtherActor :type Actor%20Object%20Reference)))

(event EventTick
  (params (DeltaSeconds :type Float%20%28single-precision%29)))

(event Input|KeyboardEvents|DebugKeyT
  (params (Key :type Key%20Structure :default "None") (ActionValue :type Input%20Action%20Value%20Structure))
  (:Pressed
    (Abilities|TryActivateAbilitybyClass (Variables|Default|GetAbilitySystem) "/Game/ComponentSystems/Magic/Farming/BP_WaterSpell.BP_WaterSpell_C" true)))

(event Input|KeyboardEvents|DebugKeyR
  (params (Key :type Key%20Structure :default "None") (ActionValue :type Input%20Action%20Value%20Structure))
  (:Pressed
    (Abilities|TryActivateAbilitybyClass (Variables|Default|GetAbilitySystem) "/Game/ComponentSystems/Magic/Farming/BP_HarvestSpell.BP_HarvestSpell_C" true)))

(event Input|KeyboardEvents|DebugKeyF
  (params (Key :type Key%20Structure :default "None") (ActionValue :type Input%20Action%20Value%20Structure))
  (bind _returnvalue (Game|GetPlayerController 0))
  (bind _returnvalue_2 (Game|GetPlayerController 0))
  ;[1 1 1] For opening the spellbook
  (:Pressed
    (if (not (Variables|Default|GetbInventoryOpen))
      (if (Variables|Default|GetbSpellBookOpen)
        (Widget|RemovefromParent (Variables|Default|GetSpellBook))
        (Input|SetInputModeGameOnly _returnvalue false)
        (Variables|/Script/Engine.PlayerController|SetbShowMouseCursor _returnvalue false)
        (Variables|Default|SetbSpellBookOpen false)
        (else
          (Utilities|IsValid (Variables|Default|GetSpellBook)
            (:Is%20Valid
              _)
            (:Is%20Not%20Valid
              (bind _returnvalue_3 (UserInterface|CreateWidget "/Game/Widgets/Spells/WBP_SpellBook.WBP_SpellBook_C"))
              (bind _output_get (Variables|Default|SetSpellBook _returnvalue_3))))
          (UserInterface|Viewport|AddtoViewport _output_get 0)
          (Input|SetInputModeGameandUI _returnvalue_2 _output_get "DoNotLock" true false)
          (Variables|/Script/Engine.PlayerController|SetbShowMouseCursor _returnvalue_2 true)
          (Variables|Default|SetbSpellBookOpen true))))))

(fn ConstructionScript)